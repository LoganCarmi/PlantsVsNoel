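; Base plant actor for a Plants vs. Zombies-style game, covering idle animation, shooting and health.
; StartIdleAnimation loops animations by plant type and flags Peashooter and Repeater as shooters with single or double shots.
; Externally toggled shooting recurses through delays, spawning pea projectiles for ShootManager.
; Overlapping zombies halt and start recurring damage scaled by attacker count; at zero HP, zombies resume and the placement widget removes the plant.
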(event OnComponentBeginOverlap(BC_Hitbox)
  (params (OverlappedComponent :type Primitive%20Component%20Object%20Reference) (OtherActor :type Actor%20Object%20Reference) (OtherComp :type Primitive%20Component%20Object%20Reference) (OtherBodyIndex :type Integer) (bFromSweep :type Boolean) (SweepResult :type Hit%20Result%20Structure%20%28by%20ref%29))
  (bind _zombiesdamaging (Variables|Default|GetZombiesDamaging))
  (bind _asbp_zombie (Utilities|Casting|CastToBP_Zombie OtherActor))
  (if (Utilities|Array|ContainsItem (Variables|Default|GetZombiesDamaging) _asbp_zombie)
    _
    (else
      (Utilities|Array|Add _zombiesdamaging _asbp_zombie)))
  (Class|ZombiesWavesGenerator|StopMovement (Variables|Default|GetZombiesWavesGenerator) _asbp_zombie)
  (CallFunction|TakeDamage (* (Utilities|Array|Length _zombiesdamaging) 70))
  (Utilities|FlowControl|Delay 0.3)
  (CallFunction|CheckforApplyingDamage))

(event Custom|CheckForApplyingDamage
  (bind _zombiesdamaging (Variables|Default|GetZombiesDamaging))
  (bind _asbp_zombie (Utilities|Casting|CastToBP_Zombie (stale OnComponentBeginOverlap(BC_Hitbox) OtherActor)))
  (if (Utilities|Array|ContainsItem (Variables|Default|GetZombiesDamaging) _asbp_zombie)
    _
    (else
      (Utilities|Array|Add _zombiesdamaging _asbp_zombie)))
  (Class|ZombiesWavesGenerator|StopMovement (Variables|Default|GetZombiesWavesGenerator) _asbp_zombie)
  (CallFunction|TakeDamage (* (Utilities|Array|Length _zombiesdamaging) 70))
  (Utilities|FlowControl|Delay 0.3)
  (CallFunction|CheckforApplyingDamage))

(event Custom|StartIdleAnimation
  (params (CorrespondingPlant :type E_PlantsSelection%20Enum :default "NewEnumerator10"))
  (bind _sm_plant (Variables|Default|GetSM_Plant))
  (CallFunction|CheckShootingPlant CorrespondingPlant)
  (Utilities|FlowControl|Delay 1.0)
  (switch Utilities|FlowControl|Switch|SwitchonE_PlantsSelection CorrespondingPlant
    (:NewEnumerator2
      (Components|Animation|PlayAnimation _sm_plant (Utilities|Array|Get(acopy) (Variables|Default|GetIdleAnimationArray)) true))
    (:NewEnumerator3
      (Components|Animation|PlayAnimation _sm_plant (Utilities|Array|Get(acopy) (Variables|Default|GetIdleAnimationArray) 1) true))
    (:NewEnumerator1
      (Components|Animation|PlayAnimation _sm_plant (Utilities|Array|Get(acopy) (Variables|Default|GetIdleAnimationArray) 2) true))
    (:NewEnumerator4
      (Components|Animation|PlayAnimation _sm_plant (Utilities|Array|Get(acopy) (Variables|Default|GetIdleAnimationArray) 3) true))
    (:NewEnumerator5
      (Components|Animation|PlayAnimation _sm_plant (Utilities|Array|Get(acopy) (Variables|Default|GetIdleAnimationArray) 4) true))
    (:NewEnumerator0
      (Components|Animation|PlayAnimation _sm_plant (Utilities|Array|Get(acopy) (Variables|Default|GetIdleAnimationArray) 5) true))
    (:NewEnumerator6
      (Components|Animation|PlayAnimation _sm_plant (Utilities|Array|Get(acopy) (Variables|Default|GetIdleAnimationArray) 6) true))
    (:NewEnumerator7
      (Components|Animation|PlayAnimation _sm_plant (Utilities|Array|Get(acopy) (Variables|Default|GetIdleAnimationArray) 7) true))
    (:NewEnumerator8
      (Components|Animation|PlayAnimation _sm_plant (Utilities|Array|Get(acopy) (Variables|Default|GetIdleAnimationArray) 8) true))))

(event Custom|StartShooting
  (if (not (Variables|Default|GetShootingMode))
    (Variables|Default|SetShootingMode true)
    (CallFunction|ShootEvent)))

(event Custom|ShootEvent
  (if (Variables|Default|GetShootingMode)
    (CallFunction|Shoot)
    (if (== (Variables|Default|GetShootRate) 2)
      (Utilities|FlowControl|Delay 0.2)
      (CallFunction|Shoot)
      (Utilities|FlowControl|Delay 1.3)
      (CallFunction|ShootEvent)
      (else
        (Utilities|FlowControl|Delay 1.5)
        (CallFunction|ShootEvent)))))

(event Custom|StopShooting
  (if (Variables|Default|GetShootingMode)
    (Variables|Default|SetShootingMode false)))

(event EventBeginPlay
  (bind _returnvalue (Actor|GetActorOfClass "/Game/Blueprints/MyZombiesWavesGenerator.MyZombiesWavesGenerator_C"))
  (Variables|Default|SetZombiesWavesGenerator _returnvalue)
  (bind _returnvalue_2 (Actor|GetActorOfClass "/Game/Blueprints/MyShootManager.MyShootManager_C"))
  (Variables|Default|SetShootManager _returnvalue_2))

(fn ConstructionScript)

(fn TakeDamage
  (params (DamageTaken :type Integer))
  (bind _zombiesdamaging (Variables|Default|GetZombiesDamaging))
  (bind _output_get (Variables|Default|SetHP (- (Variables|Default|GetHP) DamageTaken)))
  (if (<= _output_get 0)
    (for (_array_element _array_index) (Variables|Default|GetZombiesDamaging)
      (Utilities|IsValid _array_element
        (:Is%20Valid
          (Class|ZombiesWavesGenerator|RestartMovement (Variables|Default|GetZombiesWavesGenerator) _array_element))
        (:Is%20Not%20Valid
          (Utilities|Array|RemoveItem _zombiesdamaging (Utilities|Array|Get(acopy) _zombiesdamaging _array_index)))))
    (bind _returnvalue (Actor|GetActorOfClass "/Game/Blueprints/BP_WorldSpaceWidget.BP_WorldSpaceWidget_C"))
    (bind _aswbp_placement (Utilities|Casting|CastToWBP_Placement (UserInterface|GetWidget (Variables|/Game/Blueprints/BP_WorldSpaceWidget.BP_WorldSpaceWidget_C|GetWidget _returnvalue))))
    (bind _index (Default|GetIndexfromLocation _aswbp_placement (Transformation|GetWorldLocation (Variables|Default|GetSM_Plant))))
    (Default|RemovePlantatSelectedPlace _aswbp_placement _index)))

(fn CheckShootingPlant
  (params (PlantType :type E_PlantsSelection%20Enum :default "NewEnumerator10"))
  (switch Utilities|FlowControl|Switch|SwitchonE_PlantsSelection PlantType
    (:NewEnumerator1
      (Variables|Default|SetIsShootingPlant true)
      (Variables|Default|SetShootRate 1))
    (:NewEnumerator4
      (Variables|Default|SetIsShootingPlant true)
      (Variables|Default|SetShootRate 2))))

(fn Shoot
  (bind _sm_plant (Variables|Default|GetSM_Plant))
  (bind _sm_plant_2 (Variables|Default|GetSM_Plant))
  (bind _returnvalue (Transformation|GetWorldLocation _sm_plant))
  (bind _returnvalue_2 (Transformation|GetWorldLocation _sm_plant_2))
  (bind _returnvalue_3 (Game|SpawnActorfromClass "/Game/Blueprints/BP_Projectile.BP_Projectile_C" (Math|Transform|MakeTransform (Math|Vector|MakeVector (.x _returnvalue_2) (.y _returnvalue_2) 1.1e+02) "0, 0, 0" "0.700000,0.700000,0.700000") "Undefined" "MultiplyWithRoot" 0 0))
  (Components|StaticMesh|SetStaticMesh (Variables|/Game/Blueprints/BP_Projectile.BP_Projectile_C|GetProjectileStaticMesh _returnvalue_3) "/Game/Plantes/PistoPois/Projectile_PistoPois.Projectile_PistoPois")
  (Rendering|Material|SetMaterial (Variables|/Game/Blueprints/BP_Projectile.BP_Projectile_C|GetProjectileStaticMesh _returnvalue_3) 0 "/Game/Plantes/PistoPois/MI_PistoPois_Projectile.MI_PistoPois_Projectile")
  (Class|ShootManager|ShootProjectile (Variables|Default|GetShootManager) _returnvalue_3 (Math|Vector|MakeVector (.x _returnvalue) (.y _returnvalue) 1.1e+02)))