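; BP_Sun is a collectible sun actor whose interaction runs through a WBP_SunInteraction widget hosted on its Widget component.
; On BeginPlay it hands that widget a reference to itself.
; DespawnSun destroys the actor after a fixed delay if it is still valid, while DestroyCollectedSun destroys it immediately.
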(event Custom|DespawnSun
  (Utilities|FlowControl|Delay 8.0)
  (Utilities|IsValid self
    (:Is%20Valid
      (Actor|DestroyActor))))

(event EventBeginPlay
  (bind _aswbp_sun_interaction (Utilities|Casting|CastToWBP_SunInteraction (UserInterface|GetWidget (Variables|Default|GetWidget))))
  (Variables|/Game/Blueprints/WBP_SunInteraction.WBP_SunInteraction_C|SetSunParent_ref _aswbp_sun_interaction self))

(fn ConstructionScript)

(fn DestroyCollectedSun
  (Actor|DestroyActor))