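; Timed generator that keeps spawning scaled-down BP_Sun actors and gliding each one to a target position.
; RespawnSun starts on BeginPlay, picks a random spawn point, moves the sun, waits ten seconds, then calls itself again.
; The spawn point's array index selects a block of five targets, and the target's slot sets travel time.
; Both random picks exclude the last entry, since RandomInteger's maximum is exclusive.
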(event Custom|RespawnSun
  (bind _randomspawnlocation (CallFunction|GetRandomSpawnLocation))
  (bind _returnvalue (Game|SpawnActorfromClass "/Game/Blueprints/BP_Sun.BP_Sun_C" (Math|Transform|MakeTransform _randomspawnlocation "0, 0, 0" "0.400000,0.400000,0.400000") "Undefined" "MultiplyWithRoot" 0 0))
  (bind (_randomtargetlocation _over_time) (CallFunction|GetRandomTargetLocation _returnvalue))
  (Components|MoveComponentTo (Variables|/Game/Blueprints/BP_Sun.BP_Sun_C|GetDefaultSceneRoot _returnvalue) _randomtargetlocation "0, 0, 0" false false _over_time false)
  (Utilities|FlowControl|Delay 1e+01)
  (CallFunction|RespawnSun))

(event EventBeginPlay
  (bind _randomspawnlocation (CallFunction|GetRandomSpawnLocation))
  (bind _returnvalue (Game|SpawnActorfromClass "/Game/Blueprints/BP_Sun.BP_Sun_C" (Math|Transform|MakeTransform _randomspawnlocation "0, 0, 0" "0.400000,0.400000,0.400000") "Undefined" "MultiplyWithRoot" 0 0))
  (bind (_randomtargetlocation _over_time) (CallFunction|GetRandomTargetLocation _returnvalue))
  (Components|MoveComponentTo (Variables|/Game/Blueprints/BP_Sun.BP_Sun_C|GetDefaultSceneRoot _returnvalue) _randomtargetlocation "0, 0, 0" false false _over_time false)
  (Utilities|FlowControl|Delay 1e+01)
  (CallFunction|RespawnSun))

(fn ConstructionScript)

(fn GetRandomSpawnLocation
  (return (Utilities|Array|Get(acopy) (Variables|Default|GetSpawnLocationsArray) (Math|Random|RandomInteger (- (Utilities|Array|Length (Variables|Default|GetSpawnLocationsArray)) 1)))))

(fn GetRandomTargetLocation
  (params (SpawnedSun :type BP%20Sun%20Object%20Reference))
  (bind _output_get (LocalVariables|SetRandomGenerated (+ (* (Utilities|Array|FindItem (Variables|Default|GetSpawnLocationsArray) (Transformation|GetWorldLocation (Variables|/Game/Blueprints/BP_Sun.BP_Sun_C|GetDefaultSceneRoot SpawnedSun))) 5) (Math|Random|RandomInteger 4))))
  (return (Utilities|Array|Get(acopy) (Variables|Default|GetTargetLocationsArray) _output_get) (+ (Math|Integer|%(Integer) _output_get 5) 5)))