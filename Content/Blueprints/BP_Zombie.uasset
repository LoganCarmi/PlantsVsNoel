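; BP_Zombie is a lane enemy that takes damage, dies and reports to the wave generator.
; When its HitBox overlaps a BP_DetectZombie, it joins that detector's lane list and triggers shooting.
; TakeDamage lowers HP; at zero it has the detector recheck the lane, removes the hitbox and plays the death animation.
; After a short delay it destroys itself and, on the last wave, calls LastWaveChecker.
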(event OnComponentBeginOverlap(HitBox)
  (params (OverlappedComponent :type Primitive%20Component%20Object%20Reference) (OtherActor :type Actor%20Object%20Reference) (OtherComp :type Primitive%20Component%20Object%20Reference) (OtherBodyIndex :type Integer) (bFromSweep :type Boolean) (SweepResult :type Hit%20Result%20Structure%20%28by%20ref%29))
  (bind _asbp_detect_zombie (Utilities|Casting|CastToBP_DetectZombie OtherActor))
  (Utilities|Array|Add (Variables|/Game/Blueprints/BP_DetectZombie.BP_DetectZombie_C|GetZombiesOnLane _asbp_detect_zombie) self)
  (Variables|Default|SetDetectZombie_ref _asbp_detect_zombie)
  (Default|StartShooting _asbp_detect_zombie))

(event Custom|DestroyEvent
  (Utilities|FlowControl|Delay 1.0)
  (Actor|DestroyActor)
  (bind _returnvalue (Actor|GetActorOfClass "/Game/Blueprints/MyZombiesWavesGenerator.MyZombiesWavesGenerator_C"))
  (if (Variables|/Game/Blueprints/MyZombiesWavesGenerator.MyZombiesWavesGenerator_C|GetLastWave _returnvalue)
    (Default|LastWaveChecker _returnvalue)))

(fn ConstructionScript)

(fn TakeDamage
  (params (DamageTaken :type Integer))
  (bind _output_get (Variables|Default|SetHP (- (Variables|Default|GetHP) DamageTaken)))
  (if (<= _output_get 0)
    (Default|CheckZombiesonLane (Variables|Default|GetDetectZombie_ref) self)
    (Components|DestroyComponent (Variables|Default|GetHitBox))
    (Components|Animation|PlayAnimation (Variables|Default|GetSkeletalMesh) "/Game/Zombie/Animations/Death/Zombie_Animation_Death.Zombie_Animation_Death" false)
    (CallFunction|DestroyEvent)))