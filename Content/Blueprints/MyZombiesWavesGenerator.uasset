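; Zombie wave generator that runs five timed, mostly growing waves of enemies and detects victory.
; BeginPlay seeds randomness, then chains delays from DelayBetweenWaves into per-wave events that spawn zombies at random locations.
; Each wave calls its StartWave function and updates the in-game widget's announcement, with the fifth setting LastWave.
; LastWaveChecker, not called within this graph, pauses the game and shows the victory widget when no BP_Zombie actors remain.
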(event Custom|SpawnWave1
  (Class|ZombiesWavesGenerator|SpawnZombie (CallFunction|GetSpawnLocation))
  (Class|ZombiesWavesGenerator|SpawnZombie (CallFunction|GetSpawnLocation))
  (Class|ZombiesWavesGenerator|StartWave1)
  (bind _foundwidgets (Widget|GetAllWidgetsOfClass "/Game/Blueprints/WBP_IngameUI.WBP_IngameUI_C" true))
  (bind _output_get (Variables|Default|SetIngameUI (Utilities|Array|Get(acopy) _foundwidgets)))
  (Variables|/Game/Blueprints/WBP_IngameUI.WBP_IngameUI_C|SetWaveInComing _output_get "1st wave is here ! Another one is in coming..."))

(event Custom|LastWaveChecker
  (bind _outactors (Actor|GetAllActorsOfClass "/Game/Blueprints/BP_Zombie.BP_Zombie_C"))
  (if (== (Utilities|Array|Length _outactors) 0)
    (Game|SetGamePaused true)
    (bind _returnvalue (UserInterface|CreateWidget "/Game/Blueprints/WBP_Victory.WBP_Victory_C"))
    (UserInterface|Viewport|AddtoViewport _returnvalue 0)))

(event Custom|SpawnWave2
  (params (NumberOfZombies :type Integer))
  (for _index (range 1 NumberOfZombies)
    (Class|ZombiesWavesGenerator|SpawnZombie (CallFunction|GetSpawnLocation)))
  (Class|ZombiesWavesGenerator|StartWave2)
  (Variables|/Game/Blueprints/WBP_IngameUI.WBP_IngameUI_C|SetWaveInComing (Variables|Default|GetIngameUI) "2nd wave is here ! Another one is in coming..."))

(event Custom|SpawnWave5
  (params (NumberOfZombies :type Integer))
  (for _index (range 1 NumberOfZombies)
    (Class|ZombiesWavesGenerator|SpawnZombie (CallFunction|GetSpawnLocation)))
  (Class|ZombiesWavesGenerator|StartWave5)
  (Variables|Default|SetLastWave true)
  (Variables|/Game/Blueprints/WBP_IngameUI.WBP_IngameUI_C|SetWaveInComing (Variables|Default|GetIngameUI) "The last big wave is here !"))

(event Custom|SpawnWave3
  (params (NumberOfZombies :type Integer))
  (for _index (range 1 NumberOfZombies)
    (Class|ZombiesWavesGenerator|SpawnZombie (CallFunction|GetSpawnLocation)))
  (Class|ZombiesWavesGenerator|StartWave3)
  (Variables|/Game/Blueprints/WBP_IngameUI.WBP_IngameUI_C|SetWaveInComing (Variables|Default|GetIngameUI) "3rd wave is here ! Another one is in coming..."))

(event Custom|SpawnWave4
  (params (NumberOfZombies :type Integer))
  (for _index (range 1 NumberOfZombies)
    (Class|ZombiesWavesGenerator|SpawnZombie (CallFunction|GetSpawnLocation)))
  (Class|ZombiesWavesGenerator|StartWave4)
  (Variables|/Game/Blueprints/WBP_IngameUI.WBP_IngameUI_C|SetWaveInComing (Variables|Default|GetIngameUI) "4th wave is here !  One last big is in coming..."))

(event EventBeginPlay
  (bind _delaybetweenwaves (Variables|Default|GetDelayBetweenWaves))
  (Class|ZombiesWavesGenerator|InitRandomSeed)
  (Utilities|FlowControl|Delay (Utilities|Array|Get(acopy) _delaybetweenwaves))
  (CallFunction|SpawnWave1)
  (Utilities|FlowControl|Delay (Utilities|Array|Get(acopy) _delaybetweenwaves 1))
  (CallFunction|SpawnWave2 3)
  (Utilities|FlowControl|Delay (Utilities|Array|Get(acopy) _delaybetweenwaves 2))
  (CallFunction|SpawnWave3 6)
  (Utilities|FlowControl|Delay (Utilities|Array|Get(acopy) _delaybetweenwaves 3))
  (CallFunction|SpawnWave4 8)
  (Utilities|FlowControl|Delay (Utilities|Array|Get(acopy) _delaybetweenwaves 4))
  (CallFunction|SpawnWave5 11))

(fn ConstructionScript)

(fn GetSpawnLocation
  (bind _returnvalue (Class|ZombiesWavesGenerator|GetRandomIndex))
  (bind _output_get (LocalVariables|SetIndex1 _returnvalue))
  (bind _returnvalue_2 (Class|ZombiesWavesGenerator|GetRandomSpawnLocation _output_get))
  (return _returnvalue_2))